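; AI-controlled actor that runs with sound and particle effects, switching them when the run finishes.
; On BeginPlay it writes the target point and its starting location to the Blackboard and plays a collapse sound.
; Run and finish events swap the fire particle template and control audio, with finish replacing the audio reference with a second one before playing it.
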(event `self.ReceiveBeginPlay`
  (`BlackboardComponent.SetValueAsVector` (`AIBlueprintHelperLibrary.GetBlackboard` self) "Location_Point" (`self.Final Location`))
  (`BlackboardComponent.SetValueAsVector` (`AIBlueprintHelperLibrary.GetBlackboard` self) "Location_Back" (`self.K2_GetActorLocation`))
  (`GameplayStatics.PlaySoundAtLocation` "/Game/StarterContent/Audio/Collapse_Cue.Collapse_Cue" (`self.K2_GetActorLocation`) (struct) 1.0 1.0 0.0 null null null))

(event `Play_sound_and_particle_to_run`
  ;[1 1 1] Включение звука и активация партикла при беги
  (`AudioComponent.Play` (`self.Audio`) 0.0)
  (`ParticleSystemComponent.SetTemplate` (`self.ParticleSystem_Fire`) (`self.Emitter Template_1`)))

(event `Play_sound_and_particle_to_ Finish`
  ;[1 1 1] Включение звука и активация партикла при окончании бега
  (`AudioComponent.Stop` (`self.Audio`))
  (`ParticleSystemComponent.SetTemplate` (`self.ParticleSystem_Fire`) (`self.Emitter Template`))
  (bind _output_get (set `self.Audio` (`self.Audio1`)))
  (`AudioComponent.Play` _output_get 0.0))

(fn `UserConstructionScript`)